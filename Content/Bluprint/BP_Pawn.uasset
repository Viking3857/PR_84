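; BP_Pawn is a player pawn that slides sideways and spawns the BP_Ball in play.
; On BeginPlay, SpawnBall creates a ball at the capsule's transform, stores it and binds to its OneDead event.
; MoveRight input applies a fixed swept Y offset by axis sign, independent of input magnitude and frame time.
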(event EventBeginPlay
  (CallFunction|SpawnBall))

(event Collision|EventActorBeginOverlap
  (params (OtherActor :type Actor%20Object%20Reference)))

(event EventTick
  (params (DeltaSeconds :type Float%20%28single-precision%29)))

(event Input|AxisEvents|InputAxisMoveRight
  (params (AxisValue :type Float%20%28single-precision%29))
  (if (< AxisValue 0.0)
    (Transformation|AddActorWorldOffset "0.000000,-50.000000,0.000000" true)))

(event Input|AxisEvents|InputAxisMoveRight
  (params (AxisValue :type Float%20%28single-precision%29))
  (if (> AxisValue 0.0)
    (Transformation|AddActorWorldOffset "0.000000,50.000000,0.000000" true)))

(fn ConstructionScript)

(fn SpawnBall
  (bind _returnvalue (Game|SpawnActorfromClass "/Game/Bluprint/BP_Ball.BP_Ball_C" (Transformation|GetWorldTransform (Variables|Default|GetCapsule)) "AlwaysSpawn" "MultiplyWithRoot" 0 0))
  (bind _output_get (Variables|Default|SetPlayinBall _returnvalue))
  (EventDispatchers|BindEventtoOneDead _output_get (EventDispatchers|CreateEvent :!event SpawnBall))
  (return))